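; BP_CharacterBase is a base character Blueprint that links the unarmed animation layers to its mesh on BeginPlay.
; A key 1 debug-style toggle flips the movement component's rotation mode between look direction and velocity direction.
; Temporary Tick debug draws arrows for normalized acceleration from FlowCharacterMovementComponent and for the player controller's flattened control-rotation forward vector.
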(event EventBeginPlay
  (Components|SkeletalMesh|AnimationBlueprintLinking|LinkAnimClassLayers (Variables|Character|GetMesh) "/Game/Flow/Character/Animation/ABP_UnarmedAnimLayers.ABP_UnarmedAnimLayers_C"))

(event Collision|EventActorBeginOverlap
  (params (OtherActor :type Actor%20Object%20Reference)))

(event EventTick
  (params (DeltaSeconds :type Float%20%28single-precision%29))
  (bind _returnvalue (Transformation|GetActorLocation))
  (bind _returnvalue_2 (Game|GetPlayerController 0))
  (bind _returnvalue_3 (Transformation|GetActorLocation))
  (bind _returnvalue_4 (Pawn|GetControlRotation _returnvalue_2 :!class /Script/Engine.Controller))
  ;[1 1 1] Just Temp Debug
  (bind _asflow_character_movement_component (Utilities|Casting|CastToFlowCharacterMovementComponent (Variables|Character|GetCharacterMovement)))
  (Rendering|Debug|DrawDebugArrow _returnvalue (+ _returnvalue (* (Math|Vector|Normalize (/ (Pawn|Components|CharacterMovement|GetCurrentAcceleration _asflow_character_movement_component) (Class|CharacterMovementComponent|GetMaxAcceleration _asflow_character_movement_component))) (Variables|Default|GetScale))) 2e+01 "(R=1.000000,G=0.000000,B=0.000000,A=1.000000)" 0.0 2.0)
  (Rendering|Debug|DrawDebugArrow _returnvalue_3 (+ _returnvalue_3 (* (Math|Vector|Normalize (Math|Vector|GetForwardVector (Math|Rotator|MakeRotator (.roll _returnvalue_4) 0.0 (.yaw _returnvalue_4)))) (Variables|Default|GetScale))) 2e+01 "(R=1.000000,G=0.890353,B=0.024998,A=1.000000)" 0.0 5.0))

(event Input|KeyboardEvents|1
  (params (Key :type Key%20Structure :default "None"))
  (bind _charactermovement (Variables|Character|GetCharacterMovement))
  ;[1 1 1] Rotation Mode
  (:Pressed
    (Utilities|FlowControl|FlipFlop
      (:A
        (Class|FlowCharacterStateInterface|SetRotationMode(Message) _charactermovement "LookDirection"))
      (:B
        (Class|FlowCharacterStateInterface|SetRotationMode(Message) _charactermovement "VelocityDirection")))))

(fn ConstructionScript)